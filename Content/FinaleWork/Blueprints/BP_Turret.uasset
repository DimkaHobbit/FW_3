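; BP_Turret is a gun turret that sweeps back and forth, then tracks and shoots the player once detected.
; A Timeline drives the Patrol sweep, while Tick switches between Patrol and a Shoot state that yaws toward the player.
; Forward sphere traces handle detection and hits, with damage followed by a cooldown timer.
; Turrets without their own flashlight have the spotlight off and only detect players whose flashlight is on.
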(event `self.ReceiveBeginPlay`
  (bind _output_get (set `self.CurrentRotation` (`SceneComponent.K2_GetComponentRotation` (`self.SK_FPGun`))))
  (bind _output_get_2 (set `self.StartRotation` _output_get))
  (bind _output_get_3 (set `self.EndRotation` (`KismetMathLibrary.MakeRotator` (.roll _output_get_2) (.pitch _output_get_2) (+ (.yaw _output_get_2) (`self.RotationDegree`)))))
  (set `self.TargetRotation` _output_get_3)
  (`self.StartPatrol`)
  (if (not (`self.whithFlashlight`))
    (`LightComponent.SetIntensity` (`self.SpotLight`) 0.0)
    (`GameplayStatics.SpawnSoundAtLocation` "/Game/FinaleWork/Art/Sounds/A_TurretRotation.A_TurretRotation" (`SceneComponent.K2_GetComponentLocation` (`self.SK_FPGun`)) (struct) 1.0 1.0 0.0 "/Game/FinaleWork/Art/Sounds/ATT_AmbientSound.ATT_AmbientSound" null)))

(event `self.ReceiveTick`
  (params (DeltaSeconds :type "Float (single-precision)"))
  (bind _sk_fpgun (`self.SK_FPGun`))
  (bind (_returnvalue_roll _returnvalue_pitch _returnvalue_yaw) (`KismetMathLibrary.BreakRotator` (`SceneComponent.K2_GetComponentRotation` _sk_fpgun)))
  (bind (_returnvalue_roll_2 _returnvalue_pitch_2 _returnvalue_yaw_2) (`KismetMathLibrary.BreakRotator` (`KismetMathLibrary.FindLookAtRotation` (`SceneComponent.K2_GetComponentLocation` _sk_fpgun) (`self.K2_GetActorLocation` (`GameplayStatics.GetPlayerCharacter` 0)))))
  (switch `/Game/FinaleWork/Core/Enums/E_TurretState` (`self.State`)
    (:`NewEnumerator0`
      (bind _isplayerfinded (`self.Player Search`))
      (if _isplayerfinded
        (`self.StopPatrol`)
        (set `self.State` "NewEnumerator1")))
    (:`NewEnumerator1`
      (`SceneComponent.K2_SetWorldRotation` _sk_fpgun (`KismetMathLibrary.RInterpTo` (`KismetMathLibrary.MakeRotator` _returnvalue_roll _returnvalue_pitch _returnvalue_yaw) (`KismetMathLibrary.MakeRotator` _returnvalue_roll _returnvalue_pitch (- _returnvalue_yaw_2 90.0)) (`GameplayStatics.GetWorldDeltaSeconds`)) false false)
      (`|ExecutionSequence`
        (:`then_0`
          (if (`self.isCanShoot`)
            (bind _isshoot (`self.Shoot`))
            ;[1 1 1] Damage
            (if _isshoot
              (bind _asbp_third_person_character (cast `/Game/ThirdPerson/Blueprints/BP_ThirdPersonCharacter` (`GameplayStatics.GetPlayerCharacter` 0)))
              (`GameplayStatics.ApplyDamage` _asbp_third_person_character (`self.Damage`))
              (`KismetSystemLibrary.K2_SetTimerDelegate` (delegate `CanShoot`) 2.0)
              (set `self.isCanShoot` false))))
        (:`then_1`
          (bind _isplayerfinded_2 (`self.Player Search`))
          (if (not _isplayerfinded_2)
            (set `self.State` "NewEnumerator0")
            (set `self.TargetRotation` (`self.EndRotation`))
            (set `self.CurrentRotation` (`SceneComponent.K2_GetComponentRotation` (`self.SK_FPGun`)))
            (set `self.DirectionMove` "Forward")
            (`self.StartPatrol`)))))))

(event `CanShoot`
  ;[1 1 1] Damage
  (set `self.isCanShoot` true))

(event `StartPatrol`
  (bind (_direction _rotatetrack) (`Timeline|Timeline` :!via `PlayFromStart` :!label _label)
    (:`Update`
      (`SceneComponent.K2_SetWorldRotation` (`self.SK_FPGun`) (`KismetMathLibrary.RLerp` (`self.CurrentRotation`) (`self.TargetRotation`) _rotatetrack) false false))
    (:`Finished`
      (switch `ETimelineDirection` (`self.DirectionMove`)
        (:`Forward`
          (set `self.DirectionMove` "Backward")
          (set `self.TargetRotation` (`self.StartRotation`))
          (set `self.CurrentRotation` (`self.EndRotation`)))
        (:`Backward`
          (set `self.DirectionMove` "Forward")
          (set `self.TargetRotation` (`self.EndRotation`))
          (set `self.CurrentRotation` (`self.StartRotation`))))
      (`self.StartPatrol`))))

(event `StopPatrol`
  (goto _label :!via `Stop`))

(fn `Player Search`
  (returns (isPlayerFinded :type Boolean))
  (bind _scene (`self.Scene`))
  (bind _returnvalue (`SceneComponent.K2_GetComponentLocation` _scene))
  (bind (_outhit _returnvalue_2) (`KismetSystemLibrary.SphereTraceSingle` _returnvalue (+ _returnvalue (* (`SceneComponent.GetForwardVector` _scene) (`self.TargetDistance`))) 30.0 "TraceTypeQuery2"))
  (if _returnvalue_2
    (bind _asbp_third_person_character (cast `/Game/ThirdPerson/Blueprints/BP_ThirdPersonCharacter` (`.HitActor` (`GameplayStatics.BreakHitResult` _outhit)))
      (:`then`
        (if (`self.whithFlashlight`)
          (return true)
          (elif (`/Game/ThirdPerson/Blueprints/BP_ThirdPersonCharacter.isFlashfightActive` _asbp_third_person_character)
            (return true)
            (else
              (return false)))))
      (:`CastFailed`
        (return false)))
    (else
      (return false))))

(fn `Shoot`
  (returns (isShoot :type Boolean))
  (bind _returnvalue (`KismetMathLibrary.RandomFloatInRange` 0.8 1.0))
  (bind _scene (`self.Scene`))
  (bind _returnvalue_2 (`SceneComponent.K2_GetComponentLocation` _scene))
  (bind _returnvalue_3 (`SceneComponent.K2_GetComponentLocation` (`self.Scene`)))
  (bind (_outhit _returnvalue_4) (`KismetSystemLibrary.SphereTraceSingle` _returnvalue_2 (+ _returnvalue_2 (* (`SceneComponent.GetForwardVector` _scene) (`self.TargetDistance`))) 30.0 "TraceTypeQuery2"))
  (`|ExecutionSequence`
    (:`then_0`
      (`GameplayStatics.PlaySoundAtLocation` "/Game/StarterContent/Audio/A_Explosion02.A_Explosion02" _returnvalue_3 (struct) _returnvalue _returnvalue 0.0 null null null null)
      (`GameplayStatics.SpawnEmitterAtLocation` "/Game/StarterContent/Particles/P_Explosion.P_Explosion" _returnvalue_3))
    (:`then_1`
      (if _returnvalue_4
        (bind _asbp_third_person_character (cast `/Game/ThirdPerson/Blueprints/BP_ThirdPersonCharacter` (`.HitActor` (`GameplayStatics.BreakHitResult` _outhit)))
          (:`then`
            (if (`self.whithFlashlight`)
              (return true)
              (elif (`/Game/ThirdPerson/Blueprints/BP_ThirdPersonCharacter.isFlashfightActive` _asbp_third_person_character)
                (return true)
                (else
                  (return false)))))
          (:`CastFailed`
            (return false)))
        (else
          (return false))))))

(fn `UserConstructionScript`)