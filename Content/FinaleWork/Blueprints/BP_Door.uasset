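; BP_Door is a door actor that rotates toward a target rotation with an opening sound when interacted with.
; A Gate, opened by the Control event, filters Interact calls and closes once the timeline starts updating.
; The timeline lerps from the door's current rotation to TargetRotation each update.
; The sound spawns at the root's location only while no valid Audio reference exists.
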(event `/Game/FinaleWork/Blueprints/Interfaces/BPI_Interactable.Interact`
  (`/Engine/EditorBlueprintResources/StandardMacros.Gate` true :!label _label
    (:`Exit`
      (`|ExecutionSequence`
        (:`then_0`
          (bind (_direction _open_track) (`Timeline|Timeline` :!via `PlayFromStart`)
            (:`Update`
              (`self.K2_SetActorRotation` (`KismetMathLibrary.RLerp` (`self.K2_GetActorRotation`) (`self.TargetRotation`) _open_track))
              (goto _label :!via `Close`))))
        (:`then_1`
          (`self.Audio`
            (:`then`)
            (:`else`
              (bind _returnvalue (`GameplayStatics.SpawnSoundAtLocation` "/Game/FinaleWork/Art/Sounds/A_DoopOpen.A_DoopOpen" (`SceneComponent.K2_GetComponentLocation` (`self.DefaultSceneRoot`)) (struct) 1.0 1.0 0.0 "/Game/FinaleWork/Art/Sounds/ATT_AmbientSound.ATT_AmbientSound" null))
              (set `self.Audio` _returnvalue))))))))

(event `self.Control`
  (goto _label :!via `Open`))

(fn `UserConstructionScript`
  (`parent.UserConstructionScript`))