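; BP_Gate is a gate that slides toward an open offset when its Control event fires, apparently from a player pressure plate.
; Control toggles the on-panel flag with a FlipFlop, playing or reversing a Timeline that lerps the gate's height.
; Once fully open, the gate ignores Control, plays a 2D timer sound for a short delay, then closes automatically and unlocks when shut.
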(event `self.ReceiveBeginPlay`
  (bind _returnvalue (`self.K2_GetActorLocation`))
  (`parent.ReceiveBeginPlay`)
  (set `self.PlaceWhenClosed` _returnvalue)
  (set `self.CurrentPositionZ` (.z _returnvalue))
  (bind _returnvalue_2 (`GameplayStatics.CreateSound2D` "/Game/FinaleWork/Art/Sounds/A_Timer.A_Timer" 1.0 1.0 0.0 null false false))
  (set `self.TimerAudio` _returnvalue_2))

(event `self.Control`
  ;[1 1 1] Проверка игрока на плите
  (bind _isa (`/Engine/EditorBlueprintResources/StandardMacros.FlipFlop`)
    (:`A`
      _)
    (:`B`
      _))
  (set `self.IsPlayerOnPanel` _isa)
  (if (`self.IsBusy`)
    _
    (elif (`self.IsPlayerOnPanel`)
      (bind (_direction _opentrack) (`Timeline|Timeline` :!label _label)
        (:`Update`
          (`self.K2_SetActorLocation` (`KismetMathLibrary.MakeVector` (.x (+ (`self.PlaceWhenOpened`) (`self.PlaceWhenClosed`))) (.y (+ (`self.PlaceWhenOpened`) (`self.PlaceWhenClosed`))) (`KismetMathLibrary.Lerp` (`self.CurrentPositionZ`) (.z (+ (`self.PlaceWhenOpened`) (`self.PlaceWhenClosed`))) _opentrack))))
        (:`Finished`
          (switch `ETimelineDirection` _direction
            (:`Forward`
              (set `self.IsBusy` true)
              (`AudioComponent.Play` (`self.TimerAudio`) 0.0)
              (`KismetSystemLibrary.K2_SetTimerDelegate` (delegate `Open/Close`) 3.0))
            (:`Backward`
              (set `self.IsBusy` false)))))
      (else
        (goto _label :!via `Reverse`)))))

(event `Open/Close`
  (`AudioComponent.Stop` (`self.TimerAudio`))
  (goto _label :!via `Reverse`))

(fn `Open`)

(fn `UserConstructionScript`
  (`parent.UserConstructionScript`))