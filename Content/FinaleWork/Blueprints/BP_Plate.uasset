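; BP_Plate is a pressure plate that triggers a linked ControledActor when the third-person character steps on or off it.
; Box begin and end overlaps both call Control on that actor if valid, so the target receives the same call each way.
; A lever sound plays for any overlapping actor before the character check, lower-pitched and with ambient attenuation on exit.
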(event `self.Box.OnComponentBeginOverlap`
  (params (OverlappedComponent :type "PrimitiveComponent Object Reference") (OtherActor :type "Actor Object Reference") (OtherComp :type "PrimitiveComponent Object Reference") (OtherBodyIndex :type Integer) (bFromSweep :type Boolean) (SweepResult :type "HitResult Structure (by ref)"))
  (`GameplayStatics.PlaySoundAtLocation` "/Game/FinaleWork/Art/Sounds/A_Lever.A_Lever" (`self.K2_GetActorLocation`) (struct) 1.0 1.0 0.0 "/Game/FinaleWork/Art/Sounds/ATT_AmbientSound.ATT_AmbientSound" null null null)
  (cast `/Game/ThirdPerson/Blueprints/BP_ThirdPersonCharacter` OtherActor)
  (bind _controledactor (`self.ControledActor`)
    (:`then`
      (`/Game/FinaleWork/Blueprints/BP_ControlActor.Control` _controledactor))
    (:`else`)))

(event `self.Box.OnComponentEndOverlap`
  (params (OverlappedComponent :type "PrimitiveComponent Object Reference") (OtherActor :type "Actor Object Reference") (OtherComp :type "PrimitiveComponent Object Reference") (OtherBodyIndex :type Integer))
  (`GameplayStatics.PlaySoundAtLocation` "/Game/FinaleWork/Art/Sounds/A_Lever.A_Lever" (`self.K2_GetActorLocation`) (struct) 1.0 0.8 0.0 "/Game/FinaleWork/Art/Sounds/ATT_AmbientSound.ATT_AmbientSound" null null null)
  (cast `/Game/ThirdPerson/Blueprints/BP_ThirdPersonCharacter` OtherActor)
  (bind _controledactor (`self.ControledActor`)
    (:`then`
      (`/Game/FinaleWork/Blueprints/BP_ControlActor.Control` _controledactor))
    (:`else`)))

(fn `UserConstructionScript`)